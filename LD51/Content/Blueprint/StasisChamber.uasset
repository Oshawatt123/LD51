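; StasisChamber is an actor that animates a chamber holding a chick mesh and breaks it open with a growing sphere once enough lasers attach.
; AttachLaser counts lasers and triggers the sphere at four, while Tick spins the shield faster per laser and can match the chick's rotation to it.
; As the sphere expands, it swaps the cylinder to a spark material, moves the chick to a marker transform, then hides and stops animating.
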(event EventTick
  (params (DeltaSeconds :type Float%20%28single-precision%29))
  (bind _chickmovetransform (Variables|Default|GetChickMoveTransform))
  (bind _sphere (Variables|Default|GetSphere))
  (bind _sphere_2 (Variables|Default|GetSphere))
  (bind _returnvalue (Transformation|GetWorldTransform _chickmovetransform))
  (bind _returnvalue_2 (Transformation|GetWorldScale _sphere_2))
  (if (Variables|Default|GetDoAnimations)
    (if (Variables|Default|GetRotateChick)
      (|UpdateChickRotation))
    (Transformation|AddWorldRotation (Variables|Default|GetShield) (Math|Rotator|MakeRotator 0.0 0.0 (* (* DeltaSeconds (Variables|Default|GetLasersAttached)) 2e+01)) false false)
    (if (Variables|Default|GetGrowSphere)
      (Rendering|SetVisibility _sphere true false)
      (Transformation|SetWorldScale3D _sphere (+ (Transformation|GetWorldScale _sphere) (* (Class|KismetMathLibrary|VectorOne) (* DeltaSeconds 1e+01))))
      (if (> (.x _returnvalue_2) 5.0)
        (Utilities|FlowControl|Sequence
          (:then_0
            (Utilities|FlowControl|DoOnce false
              (:Completed
                (Rendering|Material|SetMaterial (Variables|Default|GetCylinder) 0 "/Game/StarterContent/Particles/Materials/M_Spark.M_Spark")
                (Transformation|SetWorldLocationAndRotation (Variables|Default|GetStaticMesh) (.location _returnvalue) (.rotation _returnvalue) false false)
                (Variables|Default|SetRotateChick false))))
          (:then_1
            (if (> (.x _returnvalue_2) 2e+01)
              (Rendering|SetVisibility (Variables|Default|GetSphere) false false)
              (Variables|Default|SetDoAnimations false))))))))

(event EventBeginPlay)

(fn ConstructionScript)

(fn AttachLaser
  (bind _result (Math|Integer|IncrementInt (Variables|Default|GetLasersAttached))
    (:%20%20
      (Variables|Default|SetGrowSphere (== _result 4)))))