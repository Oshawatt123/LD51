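; Blueprint layout tool that builds a chain of deformed meshes along an editable spline, using a set material.
; The construction script adds one spline mesh component per loop index, attached to the root and bent between that point and the next using local locations and tangents.
; The loop bound is point count plus two, so it runs past the last point; a minus-two calculation sits unused.
; The event graph has no runtime logic.
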(event EventBeginPlay)

(event Collision|EventActorBeginOverlap
  (params (OtherActor :type Actor%20Object%20Reference)))

(event EventTick
  (params (DeltaSeconds :type Float%20%28single-precision%29)))

(fn ConstructionScript
  (bind _splineboiii (Variables|Default|GetSplineboiii))
  (for _index (range 0 (+ (Spline|GetNumberOfSplinePoints (Variables|Default|GetSplineboiii)) 2))
    (bind _returnvalue (AddComponent|AddSplineMeshComponent false))
    (Rendering|Material|SetMaterial _returnvalue 0 (Variables|Default|GetSplineMaterial))
    (Transformation|AttachComponentToComponent _returnvalue (Variables|Default|GetDefaultSceneRoot) "None" "KeepRelative" "KeepRelative" "KeepRelative" true)
    (SplineMesh|SetStartandEnd _returnvalue (.Location (Spline|GetLocationandTangentatSplinePoint _splineboiii _index "Local")) (.Tangent (Spline|GetLocationandTangentatSplinePoint _splineboiii _index "Local")) (.Location (Spline|GetLocationandTangentatSplinePoint _splineboiii (+ _index 1) "Local")) (.Tangent (Spline|GetLocationandTangentatSplinePoint _splineboiii (+ _index 1) "Local")) true :!class /Script/Engine.SplineMeshComponent)))