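; NotADatingSim is an interactable Blueprint in the Prison area that starts a dialogue and repositions the JoYo actor.
; Its Interact override runs the parent logic, creates a DialogueWidget and starts it with the Dialogue text.
; It then immediately teleports JoYo to JoYoSpawnTransform without waiting for the dialogue to finish.
; The event graph and construction script add no behavior of their own.
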(event EventBeginPlay
  (|CallParentFunction) ; This node is disabled and will not be called.\nDrag off pins to build functionality.
)

(event Collision|EventActorBeginOverlap
  (params (OtherActor :type Actor%20Object%20Reference))
  (|CallParentFunction OtherActor) ; This node is disabled and will not be called.\nDrag off pins to build functionality.
)

(event EventTick
  (params (DeltaSeconds :type Float%20%28single-precision%29))
  (|CallParentFunction DeltaSeconds) ; This node is disabled and will not be called.\nDrag off pins to build functionality.
)

(fn ConstructionScript
  (|CallParentFunction))

(fn Interact
  (|CallParentFunction)
  (bind _returnvalue (UserInterface|CreateWidget "/Game/Blueprint/UI/DialogueWidget.DialogueWidget_C"))
  (Default|StartText _returnvalue (Variables|Default|GetDialogue))
  (Transformation|SetActorTransform (Variables|Default|GetJoYo) (Variables|Default|GetJoYoSpawnTransform) false true))