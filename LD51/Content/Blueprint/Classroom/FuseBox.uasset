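; Classroom fuse box interactable that responds to the player supplying a fuse.
; Interact calls the parent, then checks the first-person character's HasFuse flag before hiding the Red component and enabling collision on a DialogueBox actor.
; InteractGrabbable applies the same hide and collision changes directly, without the fuse check or parent call.
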(event EventBeginPlay
  (|CallParentFunction) ; This node is disabled and will not be called.\nDrag off pins to build functionality.
)

(event Collision|EventActorBeginOverlap
  (params (OtherActor :type Actor%20Object%20Reference))
  (|CallParentFunction OtherActor) ; This node is disabled and will not be called.\nDrag off pins to build functionality.
)

(event EventTick
  (params (DeltaSeconds :type Float%20%28single-precision%29))
  (|CallParentFunction DeltaSeconds) ; This node is disabled and will not be called.\nDrag off pins to build functionality.
)

(fn ConstructionScript
  (|CallParentFunction))

(fn Interact
  (|CallParentFunction)
  (bind _asbp_first_person_character (Utilities|Casting|CastToBP_FirstPersonCharacter (Game|GetPlayerCharacter 0)))
  (if (Variables|/Game/FirstPerson/Blueprints/BP_FirstPersonCharacter.BP_FirstPersonCharacter_C|GetbHasFuse _asbp_first_person_character)
    (Development|SetHiddeninGame (Variables|Default|GetRed) true false)
    (Collision|SetActorEnableCollision (Variables|Default|GetDialogueBox) true)))

(fn InteractGrabbable
  (Development|SetHiddeninGame (Variables|Default|GetRed) true false)
  (Collision|SetActorEnableCollision (Variables|Default|GetDialogueBox) true))