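; Base Blueprint for an interactable door that opens once by playing a level sequence.
; Interact casts the player to BP_FirstPersonCharacter and calls TryOpenDoor with an always-true condition.
; TryOpenDoor plays DoorLevelSequence and sets DoorOpen to block replays; a false condition instead triggers narrator dialogue on the character saying the door can't be opened yet.
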(event EventBeginPlay
  (|CallParentFunction) ; This node is disabled and will not be called.\nDrag off pins to build functionality.
)

(event Collision|EventActorBeginOverlap
  (params (OtherActor :type Actor%20Object%20Reference))
  (|CallParentFunction OtherActor) ; This node is disabled and will not be called.\nDrag off pins to build functionality.
)

(event EventTick
  (params (DeltaSeconds :type Float%20%28single-precision%29))
  (|CallParentFunction DeltaSeconds) ; This node is disabled and will not be called.\nDrag off pins to build functionality.
)

(fn ConstructionScript
  (|CallParentFunction))

(fn Interact
  (|CallParentFunction)
  (bind _asbp_first_person_character (Utilities|Casting|CastToBP_FirstPersonCharacter (Game|GetPlayerCharacter 0)))
  (CallFunction|TryOpenDoor true _asbp_first_person_character))

(fn TryOpenDoor
  (params (Condition :type Boolean) (InputPin :type BP%20First%20Person%20Character%20Object%20Reference))
  (if Condition
    (if (not (Variables|Default|GetDoorOpen))
      (bind _returnvalue (Sequencer|Player|CreateLevelSequencePlayer (Variables|Default|GetDoorLevelSequence)))
      (Sequencer|Player|Play _returnvalue :!class /Script/MovieScene.MovieSceneSequencePlayer)
      (Variables|Default|SetDoorOpen true))
    (else
      (Default|StartNarratorDialogue InputPin (Utilities|Struct|MakeDialogueText "Doesn't look like you can open this right now" "NewEnumerator1")))))