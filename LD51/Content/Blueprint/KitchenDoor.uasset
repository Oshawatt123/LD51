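; KitchenDoor is an interactable door that only opens when the player has the kitchen key.
; Its Interact override calls the parent, then checks HasKitchenKey on the player's BP_FirstPersonCharacter.
; With the key, it plays the PrisonDoor level sequence once, using a DoorOpen flag to block replays.
; Without it, the character's narrator dialogue reports that the door is locked.
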(event EventBeginPlay
  (|CallParentFunction) ; This node is disabled and will not be called.\nDrag off pins to build functionality.
)

(event Collision|EventActorBeginOverlap
  (params (OtherActor :type Actor%20Object%20Reference))
  (|CallParentFunction OtherActor) ; This node is disabled and will not be called.\nDrag off pins to build functionality.
)

(event EventTick
  (params (DeltaSeconds :type Float%20%28single-precision%29))
  (|CallParentFunction DeltaSeconds) ; This node is disabled and will not be called.\nDrag off pins to build functionality.
)

(fn ConstructionScript
  (|CallParentFunction))

(fn Interact
  (|CallParentFunction)
  (bind _asbp_first_person_character (Utilities|Casting|CastToBP_FirstPersonCharacter (Game|GetPlayerCharacter 0)))
  (if (Variables|/Game/FirstPerson/Blueprints/BP_FirstPersonCharacter.BP_FirstPersonCharacter_C|GetbHasKitchenKey _asbp_first_person_character)
    (if (not (Variables|Default|GetDoorOpen))
      (bind _returnvalue (Sequencer|Player|CreateLevelSequencePlayer "/Game/LevelSequences/Prison/PrisonDoor.PrisonDoor"))
      (Sequencer|Player|Play _returnvalue :!class /Script/MovieScene.MovieSceneSequencePlayer)
      (Variables|Default|SetDoorOpen true))
    (else
      (Default|StartNarratorDialogue _asbp_first_person_character (Utilities|Struct|MakeDialogueText "This door is locked" "NewEnumerator0")))))