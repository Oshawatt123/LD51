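; EGGG is an actor that exposes Move, Rotate and Activate functions for external callers, with no active event logic of its own.
; Move line-traces three times the movement vector in world space with debug drawing and, if clear, applies it as a local offset.
; Rotate adds the input to the current yaw, zeroing pitch and roll.
; Activate calls Interact on Interactable actors overlapping Trigger.
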(event EventBeginPlay)

(event Collision|EventActorBeginOverlap
  (params (OtherActor :type Actor%20Object%20Reference)))

(event EventTick
  (params (DeltaSeconds :type Float%20%28single-precision%29)))

(fn ConstructionScript)

(fn Move
  (params (Movement :type Vector))
  (bind _defaultsceneroot (Variables|Default|GetDefaultSceneRoot))
  (bind _returnvalue (Transformation|GetWorldLocation _defaultsceneroot))
  (bind _returnvalue_2 (Collision|LineTraceByChannel _returnvalue (+ (* Movement 3.0) _returnvalue) "TraceTypeQuery1" false 0 "ForDuration" true "(R=1.000000,G=0.000000,B=0.000000,A=1.000000)" "(R=0.000000,G=1.000000,B=0.000000,A=1.000000)" 2.0))
  (if (not _returnvalue_2)
    (Transformation|AddLocalOffset (Variables|Default|GetDefaultSceneRoot) Movement false false)))

(fn Rotate
  (params (EulerAngles :type Float%20%28double-precision%29))
  (Transformation|SetWorldRotation (Variables|Default|GetDefaultSceneRoot) (.Rotation (Utilities|Struct|BreakEulerTransform (Utilities|Struct|MakeEulerTransform "0.000000,0.000000,0.000000" (Math|Rotator|MakeRotator 0.0 0.0 (+ EulerAngles (.yaw (.rotation (Utilities|Struct|MakeEulerTransform "0.000000,0.000000,0.000000" (Transformation|GetWorldRotation (Variables|Default|GetDefaultSceneRoot)) "1.000000,1.000000,1.000000"))))) "1.000000,1.000000,1.000000"))) false false))

(fn Activate
  (for _array_element (Collision|GetOverlappingActors (Variables|Default|GetTrigger) "/Game/Blueprint/Interactable.Interactable_C" :!class /Script/Engine.PrimitiveComponent)
    (bind _asinteractable (Utilities|Casting|CastToInteractable _array_element))
    (Default|Interact _asinteractable)))