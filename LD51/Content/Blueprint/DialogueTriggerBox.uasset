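; A trigger box actor that shows dialogue text when the first-person character enters it, with optional media playback.
; Trigger creates the dialogue widget once, guarded by a Triggered flag.
; If a MediaPlayer is set, every overlap, whatever the actor, waits a delay, adds a media widget and binds the player's MediaSound to that player.
; Collision can optionally be switched off at BeginPlay.
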(event OnComponentBeginOverlap(TriggerBox)
  (params (OverlappedComponent :type Primitive%20Component%20Object%20Reference) (OtherActor :type Actor%20Object%20Reference) (OtherComp :type Primitive%20Component%20Object%20Reference) (OtherBodyIndex :type Integer) (bFromSweep :type Boolean) (SweepResult :type Hit%20Result%20Structure%20%28by%20ref%29))
  (CallFunction|Trigger OtherActor)
  (Utilities|IsValid (Variables|IntroVideo|GetMediaPlayer)
    (:Is%20Valid
      (Utilities|FlowControl|Delay (Variables|IntroVideo|GetVideoPlayDelay))
      (bind _returnvalue (UserInterface|CreateWidget (Variables|IntroVideo|GetMediaWidget)))
      (UserInterface|Viewport|AddtoPlayerScreen _returnvalue)
      (bind _asbp_first_person_character (Utilities|Casting|CastToBP_FirstPersonCharacter (Game|GetPlayerCharacter 0)))
      (Media|MediaSoundComponent|SetMediaPlayer (Variables|/Game/FirstPerson/Blueprints/BP_FirstPersonCharacter.BP_FirstPersonCharacter_C|GetMediaSound _asbp_first_person_character) (Variables|IntroVideo|GetMediaPlayer))
      (CameraShake|Start (Variables|/Game/FirstPerson/Blueprints/BP_FirstPersonCharacter.BP_FirstPersonCharacter_C|GetMediaSound _asbp_first_person_character)))))

(event EventBeginPlay
  (if (Variables|Default|GetTurnOffCollisionOnPlay)
    (Collision|SetActorEnableCollision false)))

(event Collision|EventActorBeginOverlap
  (params (OtherActor :type Actor%20Object%20Reference)))

(event EventTick
  (params (DeltaSeconds :type Float%20%28single-precision%29)))

(fn ConstructionScript)

(fn Trigger
  (params (HitActor :type Actor%20Object%20Reference))
  (if (not (Variables|Default|GetTriggered))
    (Utilities|Casting|CastToBP_FirstPersonCharacter HitActor)
    (bind _returnvalue (UserInterface|CreateWidget "/Game/Blueprint/UI/DialogueWidget.DialogueWidget_C"))
    (Default|StartText _returnvalue (Variables|Default|GetDialogueText))
    (UserInterface|Viewport|AddtoPlayerScreen _returnvalue)
    (Variables|Default|SetTriggered true)))