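; An interactable button actor that controls the EGG actor when used.
; On BeginPlay it caches a reference to the EGGG actor found in the level.
; Its Interact override calls one action on that actor by priority: Move for a nonzero MovementVector, Rotate for a nonzero Rotation, or Activate if ActivateEGG is set.
; With none set, it prints a "No behavior defined" message.
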(event EventBeginPlay
  (|CallParentFunction)
  (bind _returnvalue (Actor|GetActorOfClass "/Game/Blueprint/EGGG.EGGG_C"))
  (Variables|Default|SetEGG _returnvalue))

(event Collision|EventActorBeginOverlap
  (params (OtherActor :type Actor%20Object%20Reference))
  (|CallParentFunction OtherActor) ; This node is disabled and will not be called.\nDrag off pins to build functionality.
)

(event EventTick
  (params (DeltaSeconds :type Float%20%28single-precision%29))
  (|CallParentFunction DeltaSeconds) ; This node is disabled and will not be called.\nDrag off pins to build functionality.
)

(fn ConstructionScript
  (|CallParentFunction))

(fn Interact
  (|CallParentFunction)
  (Utilities|IsValid (Variables|Default|GetEGG)
    (:Is%20Valid
      (if (not (== (Math|Vector|VectorLength (Variables|Default|GetMovementVector)) 0.0))
        (Default|Move (Variables|Default|GetEGG) (Variables|Default|GetMovementVector))
        (elif (not (== (Variables|Default|GetRotation) 0.0))
          (Default|Rotate (Variables|Default|GetEGG) (Variables|Default|GetRotation))
          (elif (Variables|Default|GetActivateEGG)
            (Default|Activate (Variables|Default|GetEGG))
            (else
              (Development|PrintString "No behavior defined"))))))))