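; A grabbable fuse that is consumed when dropped near a FuseBox.
; On drop, after the parent logic, it sphere-traces on the Visibility channel around its physics mesh using DropRadius.
; The first FuseBox hit receives InteractGrabbable, then the fuse destroys itself and breaks the loop to avoid repeat triggers.
; The construction script sizes a sphere component to the same DropRadius.
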(event EventBeginPlay
  (|CallParentFunction) ; This node is disabled and will not be called.\nDrag off pins to build functionality.
)

(event Collision|EventActorBeginOverlap
  (params (OtherActor :type Actor%20Object%20Reference))
  (|CallParentFunction OtherActor) ; This node is disabled and will not be called.\nDrag off pins to build functionality.
)

(event EventTick
  (params (DeltaSeconds :type Float%20%28single-precision%29))
  (|CallParentFunction DeltaSeconds) ; This node is disabled and will not be called.\nDrag off pins to build functionality.
)

(fn ConstructionScript
  (|CallParentFunction)
  (Components|Sphere|SetSphereRadius (Variables|Default|GetSphere) (Variables|Default|GetDropRadius) true))

(fn DropGrabbable
  (bind _physicsmesh (Variables|Default|GetPhysicsMesh))
  (bind _returnvalue (Transformation|GetWorldLocation _physicsmesh))
  (|CallParentFunction)
  (bind _outhits (Collision|MultiSphereTraceByChannel _returnvalue _returnvalue (Variables|Default|GetDropRadius) "TraceTypeQuery1" false 0 "None"))
  ;[1 0.06951 0] THIS NEEDS TO BREAK OTHERWISE IT WILL GO MULTPLE TIMES
  (bind _array_element (Utilities|Array|ForEachLoopwithBreak _outhits :!label _label)
    (:LoopBody
      (bind _asfuse_box (Utilities|Casting|CastToFuseBox (.HitActor (Collision|BreakHitResult _array_element))))
      (Default|InteractGrabbable _asfuse_box)
      (Actor|DestroyActor)
      (goto _label Break))))