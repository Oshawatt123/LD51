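; State manager that cycles through tagged groups of world actors, showing one state's objects at a time.
; BeginPlay gathers StateObjectBase actors into a map per StateTag, then disables every state from index 1 onward.
; SwitchState disables the current state, advances CurrentState with wraparound and enables the next, toggling actor visibility and StateMesh collision.
; Tick only prints a leftover "Hello" debug string; nothing here calls SwitchState.
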(event EventBeginPlay
  ;[1 1 1] Setup state objects map
  (for _array_element (Variables|Default|GetStateTags)
    (Utilities|Array|Clear (Variables|Default|GetTempStateObjectArray))
    (bind _outactors (Actor|GetAllActorswithTag (GameplayTags|GetTagName _array_element)))
    (for _array_element_2 _outactors
      (bind _asstate_object_base (Utilities|Casting|CastToStateObjectBase _array_element_2))
      (Utilities|Array|Add (Variables|Default|GetTempStateObjectArray) _asstate_object_base))
    (Utilities|Map|Add (Variables|Default|GetStateObjects) _array_element (Utilities|Struct|MakeStateObjects _array_element (Variables|Default|GetTempStateObjectArray))))
  ;[1 1 1] Setup states from the beginning
  (for _index (range 1 (Utilities|Array|Length (Variables|Default|GetStateTags)))
    (CallFunction|SetSpecificState false _index)))

(event EventTick
  (params (DeltaSeconds :type Float%20%28single-precision%29))
  (Development|PrintString "Hello"))

(fn ConstructionScript)

(fn SwitchState
  ;[1 1 1] Disable Old State
  (CallFunction|SetState false)
  ;[1 1 1] Increment State Safely
  (bind _result (Math|Integer|IncrementInt (Variables|Default|GetCurrentState))
    (:%20%20
      (if (>= _result (Utilities|Array|Length (Variables|Default|GetStateTags)))
        (Variables|Default|SetCurrentState 0))
      ;[1 1 1] Enable New State
      (CallFunction|SetState true))))

(fn SetState
  (params (StateActive :type Boolean))
  (bind _stateobjects (Variables|Default|GetStateObjects))
  (bind _statetags (Variables|Default|GetStateTags))
  (bind _currentstate (Variables|Default|GetCurrentState))
  (bind _output (Utilities|Array|Get(acopy) _statetags _currentstate))
  (bind (_value _returnvalue) (Utilities|Map|Find _stateobjects _output))
  ;[1 1 1] For each object in a state
  (if _returnvalue
    (for _array_element (.Objects (Utilities|Struct|BreakStateObjects _value))
      ;[1 1 1] Toggle visibility and collision
      (Rendering|SetActorHiddenInGame _array_element (not StateActive))
      (if StateActive
        (Collision|SetCollisionEnabled (Variables|/Game/Blueprint/State/StateObjectBase.StateObjectBase_C|GetStateMesh _array_element) "QueryAndPhysics")
        (else
          (Collision|SetCollisionEnabled (Variables|/Game/Blueprint/State/StateObjectBase.StateObjectBase_C|GetStateMesh _array_element) "NoCollision"))))))

(fn SetSpecificState
  (params (StateActive :type Boolean) (StateIndex :type Integer))
  (bind _stateobjects (Variables|Default|GetStateObjects))
  (bind _statetags (Variables|Default|GetStateTags))
  (bind _output (Utilities|Array|Get(acopy) _statetags StateIndex))
  (bind (_value _returnvalue) (Utilities|Map|Find _stateobjects _output))
  ;[1 1 1] For each object in a state
  (if _returnvalue
    (for _array_element (.Objects (Utilities|Struct|BreakStateObjects _value))
      ;[1 1 1] Toggle visibility and collision
      (Rendering|SetActorHiddenInGame _array_element (not StateActive))
      (if StateActive
        (Collision|SetCollisionEnabled (Variables|/Game/Blueprint/State/StateObjectBase.StateObjectBase_C|GetStateMesh _array_element) "QueryAndPhysics")
        (else
          (Collision|SetCollisionEnabled (Variables|/Game/Blueprint/State/StateObjectBase.StateObjectBase_C|GetStateMesh _array_element) "NoCollision"))))))