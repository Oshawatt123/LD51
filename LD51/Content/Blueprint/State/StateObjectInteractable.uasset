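; StateObjectInteractable is an interactable Blueprint that activates linked objects and can be gated behind a count of prior activations.
; Interact activates ObjectToEdit only once OthersActivated meets Requirements.
; Without a valid ObjectToEdit, it activates InteractableToActivate instead, falling back to starting a Timer.
; Its own Activate just increments OthersActivated, so other objects can count toward its requirement.
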(event EventBeginPlay
  (|CallParentFunction) ; This node is disabled and will not be called.\nDrag off pins to build functionality.
)

(event Collision|EventActorBeginOverlap
  (params (OtherActor :type Actor%20Object%20Reference))
  (|CallParentFunction OtherActor) ; This node is disabled and will not be called.\nDrag off pins to build functionality.
)

(event EventTick
  (params (DeltaSeconds :type Float%20%28single-precision%29))
  (|CallParentFunction DeltaSeconds) ; This node is disabled and will not be called.\nDrag off pins to build functionality.
)

(fn ConstructionScript
  (|CallParentFunction))

(fn Interact
  (bind _objecttoedit (Variables|Default|GetObjectToEdit))
  (bind _interactabletoactivate (Variables|Default|GetInteractableToActivate))
  (bind _timer (Variables|Default|GetTimer))
  (Utilities|IsValid _objecttoedit
    (:Is%20Valid
      (if (>= (Variables|Default|GetOthersActivated) (Variables|Default|GetRequirements))
        (Default|Activate _objecttoedit)))
    (:Is%20Not%20Valid
      (Utilities|IsValid _interactabletoactivate
        (:Is%20Valid
          (CallFunction|Activate _interactabletoactivate))
        (:Is%20Not%20Valid
          (Utilities|IsValid _timer
            (:Is%20Valid
              (Default|StartTimer _timer))))))))

(fn Activate
  (Math|Integer|IncrementInt (Variables|Default|GetOthersActivated)))