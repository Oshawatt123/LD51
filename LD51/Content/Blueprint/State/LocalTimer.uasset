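; LocalTimer is a countdown timer that calls SwitchState on LocalStateManager every ten seconds once started.
; StartTimer adds a new TimerWidget to the first player's screen and sets a looping event timer.
; Tick derives the remaining time from that timer's handle and pushes it to the widget as formatted text.
; StopTimer clears the timer handle but leaves the widget on screen.
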(event Custom|CustomEvent_0
  (Default|SwitchState (Variables|Default|GetLocalStateManager)))

(event Custom|StartTimer
  (bind _returnvalue (UserInterface|CreateWidget "/Game/Blueprint/UI/TimerWidget.TimerWidget_C" (Game|GetPlayerController 0)))
  (UserInterface|Viewport|AddtoPlayerScreen _returnvalue)
  (bind _returnvalue_2 (Utilities|Time|SetTimerbyEvent (delegate Custom|CustomEvent_0) 1e+01 true)))

(event Custom|StopTimer
  (Utilities|Time|ClearandInvalidateTimerbyHandle (stale Custom|StartTimer _returnvalue_2)))

(event EventTick
  (params (DeltaSeconds :type Float%20%28single-precision%29))
  (Utilities|IsValid (stale Custom|StartTimer _returnvalue)
    (:Is%20Valid
      (Default|UpdateTimer (stale Custom|StartTimer _returnvalue) (Utilities|Text|ToText(Float) (- 1e+01 (Class|KismetSystemLibrary|GetTimerElapsedTimeHandle (stale Custom|StartTimer _returnvalue_2))) "HalfToEven" false true 1 324 0 2)))))

(fn ConstructionScript)