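; Editable state object for an elevator that moves between two relative points once activated.
; The construction script builds the InterpToMovement control points from Point1 and Point2 and applies the Duration.
; Movement ticking is switched off on BeginPlay and switched on by the overridden Activate, so the elevator stays still until triggered.
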(event EventBeginPlay
  (Components|Tick|SetComponentTickEnabled (Variables|Default|GetInterpToMovement) false))

(fn ConstructionScript
  (bind _interptomovement (Variables|Default|GetInterpToMovement))
  (|CallParentFunction)
  (Variables|/Script/Engine.InterpToMovementComponent|SetControlPoints _interptomovement (Utilities|Array|MakeArray (Utilities|Struct|MakeInterpControlPoint (Variables|Default|GetPoint1) true) (Utilities|Struct|MakeInterpControlPoint (Variables|Default|GetPoint2) true)))
  (Variables|/Script/Engine.InterpToMovementComponent|SetDuration _interptomovement (Variables|Default|GetDuration)))

(fn Activate
  (|CallParentFunction)
  (Components|Tick|SetComponentTickEnabled (Variables|Default|GetInterpToMovement) true))